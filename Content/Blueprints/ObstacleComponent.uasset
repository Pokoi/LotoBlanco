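; Obstacle component that temporarily reveals its owning object when touched by a visual sound, then hides it again.
; Touched shows the owner and records whether a character spawned the sound; if the outline is already visible, only character-spawned sounds refresh it.
; A retriggerable delay hides it after VisibleTime.
; While visible, Tick applies each FirstPersonCharacter's OutlineColor to the outline through newly created dynamic material instances.
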(event Custom|Hide%20object
  (params (Owner :type Actor%20Object%20Reference))
  (Utilities|FlowControl|RetriggerableDelay (Variables|Default|GetVisible%20Time))
  (Variables|Default|Setvisible false)
  (Rendering|SetVisibility (Variables|/Script/Engine.Actor|GetRootComponent Owner) false true))

(event EventTick
  (params (DeltaSeconds :type Float%20%28single-precision%29))
  (if (Variables|Default|Getvisible)
    (bind _outactors (Actor|GetAllActorsOfClass "/Game/FirstPersonBP/Blueprints/FirstPersonCharacter.FirstPersonCharacter_C"))
    (for _array_element _outactors
      (CallFunction|SetOutlineColor (Variables|/Game/FirstPersonBP/Blueprints/FirstPersonCharacter.FirstPersonCharacter_C|Getoutline%20color _array_element) (Components|GetOwner)))))

(fn Touched
  (params (outline_color :type Linear%20Color%20Structure) (first_round :type Boolean) (visual%20sound%20spawned%20by%20character :type Boolean))
  (LocalVariables|Setowner (Components|GetOwner))
  (bind _asobject (Utilities|Casting|CastToobject (LocalVariables|Getowner)))
  (bind _output_get (LocalVariables|Setowner%20object%20reference _asobject))
  (if (Rendering|IsVisible (Variables|/Game/FirstPersonBP/Blueprints/object.object_C|Getotuline _output_get))
    (if visual%20sound%20spawned%20by%20character
      (Variables|/Game/FirstPersonBP/Blueprints/object.object_C|Setwas%20activated%20by%20character (LocalVariables|Getowner%20object%20reference) visual%20sound%20spawned%20by%20character :!label _label)
      (Rendering|SetVisibility (Variables|/Script/Engine.Actor|GetRootComponent (LocalVariables|Getowner)) true true)
      (Variables|Default|Setvisible true)
      (CallFunction|HideObject (LocalVariables|Getowner)))
    (else
      (goto _label))))

(fn SetOutlineColor
  (params (color :type Linear%20Color%20Structure) (owner :type Actor%20Object%20Reference))
  ;[0 0 0] Set the oultine color
  (bind _asobject (Utilities|Casting|CastToobject owner))
  (bind _returnvalue (Rendering|Material|CreateDynamicMaterialInstance (Variables|/Game/FirstPersonBP/Blueprints/object.object_C|Getotuline _asobject) 0 (stale _array_element) "None" :!class /Script/Engine.PrimitiveComponent))
  (Rendering|Material|SetVectorParameterValue _returnvalue "outline_color" color :!class /Script/Engine.MaterialInstanceDynamic))