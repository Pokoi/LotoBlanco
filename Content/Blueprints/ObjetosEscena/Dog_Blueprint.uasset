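; Dog scene object that periodically emits a bark as both audio and a visual sound pulse.
; A looping timer from BeginPlay spawns a VisualSound actor sized by SoundRadius and plays Perro_Cue at the dog's location.
; The FinalPhase event makes each later pulse also call Enemy on every FirstPersonCharacter.
; It also changes RateSound, but does not restart the running timer.
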(event Custom|SpawnSound
  ;[0 0 0] Spawn sound
  (bind _returnvalue (Game|SpawnActorfromClass "/Game/Blueprints/VisualSound.VisualSound_C" (Transformation|GetActorTransform) "Undefined" 0 0.0 "(R=1.000000,G=1.000000,B=1.000000,A=0.000000)" true 0))
  (Variables|/Game/Blueprints/VisualSound.VisualSound_C|SetMax%20Radius _returnvalue (Variables|Default|GetSound%20Radius))
  (Audio|SpawnSoundatLocation "/Game/sounds/Perro/Perro_Cue.Perro_Cue" (Transformation|GetActorLocation) "0, 0, 0" 1.0 1.0 0.0 0 0)
  (if (Variables|Default|Getfinal_phase)
    (bind _outactors (Actor|GetAllActorsOfClass "/Game/FirstPersonBP/Blueprints/FirstPersonCharacter.FirstPersonCharacter_C"))
    (for _array_element _outactors
      (Default|Enemy _array_element))))

(event Custom|Final%20Phase
  (Variables|Default|Setrate%20sound 5.0)
  (Variables|Default|Setfinal_phase true))

(event EventBeginPlay
  ;[0 0 0] Start
  (Utilities|Time|SetTimerbyEvent (delegate Custom|SpawnSound) (Variables|Default|Getrate%20sound) true))

(event Collision|EventActorBeginOverlap
  (params (OtherActor :type Actor%20Object%20Reference)))

(event EventTick
  (params (DeltaSeconds :type Float%20%28single-precision%29)))

(fn ConstructionScript
  (Variables|Default|Setotuline (Variables|Default|GetOutline)))